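; BP_Buttons is an interactable actor that spawns a green point light when its Interact event fires.
; Interact spawns a PointLight at the Arrow component's transform, owned by the button with the player character as instigator, then sets its intensity and color.
; Each interaction adds another light, as no reference is kept and nothing removes earlier ones.
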(event `self.ReceiveBeginPlay`
  (`parent.ReceiveBeginPlay`))

(event `self.Interact`
  (bind _returnvalue (`|SpawnActorFromClass` "/Script/Engine.PointLight" (`SceneComponent.K2_GetComponentToWorld` (`self.Arrow`)) "Undefined" "OverrideRootScale" self (`GameplayStatics.GetPlayerCharacter` 0)))
  (bind _pointlightcomponent (`PointLight.PointLightComponent` _returnvalue))
  (`LightComponent.SetIntensity` _pointlightcomponent 100.0)
  (`LightComponent.SetLightColor` _pointlightcomponent (struct :`R` 0.057281 :`G` 0.804167 :`B` 0.030156 :`A` 1.0) true))

(fn `UserConstructionScript`
  (`parent.UserConstructionScript`))