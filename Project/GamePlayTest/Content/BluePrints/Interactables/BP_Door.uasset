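; BP_Door is an interactable door that snaps open when used and closes itself after a short delay.
; BeginPlay caches the mesh's starting world rotation.
; Interact calls ToggleInteract, which sets a fixed absolute world rotation and ignores its Target input, then restores the cached rotation after the delay.
; Rotation changes are instant, as the clamped RInterpTo smoothing logic is left unconnected.
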(event `self.ReceiveBeginPlay`
  (bind (_returnvalue_location _returnvalue_rotation) (`KismetMathLibrary.BreakTransform` (`SceneComponent.K2_GetComponentToWorld` (`self.StaticMesh`))))
  (`parent.ReceiveBeginPlay`)
  (set `self.Inital Rotation` _returnvalue_rotation))

(event `ToggleInteract`
  (params (Target :type "Rotator Structure" :default (struct :`Yaw` 90.0)))
  (`SceneComponent.K2_SetWorldRotation` (`self.StaticMesh`) (struct :`Yaw` 90.0) false false))

(event `self.Interact`
  (`self.ToggleInteract` (struct :`Yaw` 90.0))
  (`KismetSystemLibrary.Delay` 2.0)
  (`SceneComponent.K2_SetWorldRotation` (`self.StaticMesh`) (`self.Inital Rotation`) false false))

(fn `UserConstructionScript`
  (`parent.UserConstructionScript`))