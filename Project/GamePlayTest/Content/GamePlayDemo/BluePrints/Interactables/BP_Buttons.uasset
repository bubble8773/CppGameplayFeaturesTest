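; BP_Buttons is an interactable button that toggles a referenced rect light on and off.
; On Interact, after a validity check and a short delay, a FlipFlop alternates between setting the light to a configurable intensity with a green color and setting its intensity to zero.
; BeginPlay jumps straight to the off branch, so the light starts dark.
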(event `self.Interact`
  (bind _rectlight (`self.RectLight`))
  (`self.RectLight`
    (:`then`
      (`KismetSystemLibrary.Delay` 0.2)
      (`/Engine/EditorBlueprintResources/StandardMacros.FlipFlop`
        (:`A`
          (`LightComponent.SetIntensity` _rectlight (`self.Intensity`))
          (`LightComponent.SetLightColor` _rectlight (struct :`R` 0.057281 :`G` 0.804167 :`B` 0.030156 :`A` 1.0) true))
        (:`B`
          (`LightComponent.SetIntensity` (`self.RectLight`) 0.0 :!label _label))))
    (:`else`)))

(event `self.ReceiveBeginPlay`
  (goto _label))

(fn `UserConstructionScript`
  (`parent.UserConstructionScript`))